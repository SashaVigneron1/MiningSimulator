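; BP_Character is a player character with axis-driven walking and horizontal turning.
; Input events cache forward and right axis values, and Tick turns them into movement input relative to the control rotation's yaw, scaled by MovementSpeed.
; An IsAllowedToMove flag, set through SetMovement, gates both movement and turning, and GetCamera exposes the Camera.
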(event EventTick
  (params (DeltaSeconds :type Float%20%28single-precision%29))
  (bind _returnvalue (Pawn|GetControlRotation :!class /Script/Engine.Pawn))
  (bind _returnvalue_2 (Pawn|GetControlRotation :!class /Script/Engine.Pawn))
  (bind _rightaxis (Variables|Default|GetrightAxis))
  (bind _forwardaxis (Variables|Default|GetforwardAxis))
  (bind _yaw (Math|Rotator|BreakRotator _returnvalue))
  (bind _yaw_2 (Math|Rotator|BreakRotator _returnvalue_2))
  (bind _returnvalue_3 (Math|Rotator|MakeRotator 0.0 0.0 _yaw))
  (bind _returnvalue_4 (Math|Rotator|MakeRotator 0.0 0.0 _yaw_2))
  (bind _returnvalue_5 (Math|Vector|GetForwardVector _returnvalue_4))
  (bind _returnvalue_6 (Math|Vector|GetRightVector _returnvalue_3))
  (bind (_x _y _z) (Math|Vector|BreakVector _returnvalue_6))
  (bind (_x_2 _y_2 _z_2) (Math|Vector|BreakVector _returnvalue_5))
  (if (Variables|Default|GetisAllowedToMove)
    (if (!= (Variables|Default|GetforwardAxis) 0.0)
      ;[1 1 1] Add Forward Movement
      (Pawn|Input|AddMovementInput (Math|Vector|MakeVector (* _x_2 _forwardaxis) (* _forwardaxis _y_2) _z_2) (Variables|Default|GetmovementSpeed) false))
    (if (!= (Variables|Default|GetrightAxis) 0.0)
      ;[1 1 1] Add Sidewards Movement
      (Pawn|Input|AddMovementInput (Math|Vector|MakeVector (* _x _rightaxis) (* _y _rightaxis) _z) (Variables|Default|GetmovementSpeed) false))))

(event Input|AxisEvents|InputAxisTurn
  (params (AxisValue :type Float%20%28single-precision%29))
  (if (Variables|Default|GetisAllowedToMove)
    (Pawn|Input|AddControllerYawInput AxisValue)))

(event Input|AxisEvents|InputAxisMovementForward
  (params (AxisValue :type Float%20%28single-precision%29))
  (Variables|Default|SetforwardAxis AxisValue))

(event Input|AxisEvents|InputAxisMovementRight
  (params (AxisValue :type Float%20%28single-precision%29))
  (Variables|Default|SetrightAxis AxisValue))

(fn ConstructionScript)

(fn GetCamera
  (return (Variables|Default|GetCamera)))

(fn SetMovement
  (params (value :type Boolean))
  (Variables|Default|SetisAllowedToMove value))