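; Game mode that runs the core loop: money balance, random power outages, game over when the balance drops below zero, and restart.
; BeginPlay creates the main and welcome widgets, links BPCMissions and caches every point light.
; Tick pushes balance to missions and alternates power on randomized timers, zeroing light intensities during outages and updating the HUD countdown.
; Helper functions adjust the balance, shorten the current power timer and reset game state.
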(event EventBeginPlay
  (Utilities|FlowControl|Sequence
    (:then_0
      ;[1 1 1] Create Widget
      (bind _returnvalue (UserInterface|CreateWidget "/Game/Blueprints/Main_Widget.Main_Widget_C"))
      (Variables|Default|SetMainWidget _returnvalue)
      (UserInterface|Viewport|AddtoViewport _returnvalue 0)
      (Default|SetBalance (Variables|Default|GetMainWidget) (Variables|Default|Getbalance))
      (Default|SetGameMode (Variables|Default|GetMainWidget) self))
    (:then_1
      (Class|BPCMissions|SetGameMode (Variables|Default|GetBPC_Missions) self))
    (:then_2
      ;[1 1 1] Set Electricity Stuff
      (bind _outactors (Actor|GetAllActorsOfClass "/Script/Engine.PointLight"))
      (Variables|Electricity|SetLightsources _outactors)
      (Variables|Electricity|SetcurrElectricityTime (Math|Random|RandomFloatinRange (Variables|Electricity|GetminTimeBeforeElectricityOff) (Variables|Electricity|GetmaxTimeBeforeElectricityOff))))
    (:then_3
      ;[1 1 1] Background Noise
      (Audio|PlaySoundatLocation "/Game/Sounds/ComputerOn.ComputerOn" (Transformation|GetWorldLocation (Variables|Default|GetDefaultSceneRoot)) "0, 0, 0" 0.3 1.0 0.0 0 0 0))
    (:then_4
      (bind _returnvalue_2 (UserInterface|CreateWidget "/Game/Blueprints/WelcomeWidget.WelcomeWidget_C"))
      (bind _output_get (Variables|Default|SetWelcomeWidget _returnvalue_2))
      (UserInterface|Viewport|AddtoViewport _output_get 0)
      (Input|EnableInput (Game|GetPlayerController 0)))))

(event EventTick
  (params (DeltaSeconds :type Float%20%28single-precision%29))
  (if (not (Variables|Default|GetisGameOver))
    (Utilities|FlowControl|Sequence
      (:then_0
        ;[1 1 1] Set Missions
        (Class|BPCMissions|SetBalance (Variables|Default|GetBPC_Missions) (Variables|Default|Getbalance)))
      (:then_1
        ;[1 1 1] Handle Electricity
        (if (Variables|Electricity|GetisElectricityOn)
          (bind _output_get (Variables|Electricity|SetaccElectricityTime (+ (Variables|Electricity|GetaccElectricityTime) DeltaSeconds)))
          (if (> _output_get (Variables|Electricity|GetcurrElectricityTime))
            (Variables|Electricity|SetisElectricityOn false)
            (Variables|Electricity|SetaccElectricityTime 0.0)
            (Variables|Electricity|SetcurrElectricityTime (Math|Random|RandomFloatinRange (Variables|Electricity|GetminTimeBeforeElectricityOn) (Variables|Electricity|GetmaxTimeBeforeElectricityOn)))
            (CallFunction|SetLightSourcesActive false)
            (Variables|/Game/Blueprints/Main_Widget.Main_Widget_C|SetisPowerOff (Variables|Default|GetMainWidget) true)
            (Audio|PlaySound2D "/Game/Sounds/PowerDown.PowerDown" 1.0 1.0 0.0 0 0))
          (else
            (bind _output_get_2 (Variables|Electricity|SetaccElectricityTime (+ (Variables|Electricity|GetaccElectricityTime) DeltaSeconds)))
            (Variables|/Game/Blueprints/Main_Widget.Main_Widget_C|SetPowerOffTimeLeft (Variables|Default|GetMainWidget) (- (Variables|Electricity|GetcurrElectricityTime) (Variables|Electricity|GetaccElectricityTime)))
            (if (> _output_get_2 (Variables|Electricity|GetcurrElectricityTime))
              (Variables|Electricity|SetisElectricityOn true)
              (Variables|Electricity|SetaccElectricityTime 0.0)
              (Variables|Electricity|SetcurrElectricityTime (Math|Random|RandomFloatinRange (Variables|Electricity|GetminTimeBeforeElectricityOff) (Variables|Electricity|GetmaxTimeBeforeElectricityOff)))
              (CallFunction|SetLightSourcesActive true)
              (Variables|/Game/Blueprints/Main_Widget.Main_Widget_C|SetisPowerOff (Variables|Default|GetMainWidget) false)
              (Audio|PlaySound2D "/Game/Sounds/PowerOn.PowerOn" 1.0 1.0 0.0 0 0)))))
      (:then_2
        ;[1 1 1] Check Game Over
        (if (< (Variables|Default|Getbalance) 0.0)
          (bind _output_get_3 (Variables|Default|SetisGameOver true))
          (Variables|/Game/Blueprints/Main_Widget.Main_Widget_C|SetisGameOver (Variables|Default|GetMainWidget) _output_get_3)
          (Class|BPCMissions|SetGameOver (Variables|Default|GetBPC_Missions) true)
          (Audio|PlaySound2D "/Game/Sounds/GameOver.GameOver" 1.0 1.0 0.0 0 0)
          (Variables|/Script/Engine.PlayerController|SetbShowMouseCursor (Game|GetPlayerController 0) true)))
      (:then_3
        ;[1 1 1] Electricity Time left
        (if (<= (Variables|Electricity|GetaccPowerTimeDecreasing) 0.2)
          (Variables|Electricity|SetaccPowerTimeDecreasing (+ (Variables|Electricity|GetaccPowerTimeDecreasing) DeltaSeconds))
          (else
            (Variables|/Game/Blueprints/Main_Widget.Main_Widget_C|SetisPowerTimeDecreasing (Variables|Default|GetMainWidget) false)))))))

(event Input|ActionEvents|InputActionShowInfo
  (params (Key :type Key%20Structure :default "None"))
  (bind _welcomewidget (Variables|Default|GetWelcomeWidget))
  (:Pressed
    (if (not (Variables|/Game/Blueprints/WelcomeWidget.WelcomeWidget_C|GetisShowing _welcomewidget))
      (Default|Show _welcomewidget true))))

(event Input|ActionEvents|InputActionResetCamera
  (params (Key :type Key%20Structure :default "None"))
  (bind _welcomewidget (Variables|Default|GetWelcomeWidget))
  (:Pressed
    (if (Variables|/Game/Blueprints/WelcomeWidget.WelcomeWidget_C|GetisShowing _welcomewidget)
      (Default|Show _welcomewidget false))))

(fn ConstructionScript)

(fn AddBalance
  (params (value :type Float%20%28single-precision%29))
  (bind _output_get (Variables|Default|Setbalance (+ value (Variables|Default|Getbalance))))
  (Default|SetBalance (Variables|Default|GetMainWidget) _output_get))

(fn SetMissionBalance
  (bind _returnvalue (Class|BPCMissions|GetBalance (Variables|Default|GetBPC_Missions)))
  (Variables|Default|Setbalance _returnvalue))

(fn SetUIVisibility
  (params (Visibility :type Boolean))
  (Default|SetUIVisibility (Variables|Default|GetMainWidget) Visibility))

(fn RestartGame
  (bind _mainwidget (Variables|Default|GetMainWidget))
  (Class|BPCMissions|ResetGame (Variables|Default|GetBPC_Missions))
  (bind _output_get (Variables|Default|Setbalance 9999.0))
  (Default|SetBalance (Variables|Default|GetMainWidget) _output_get)
  (Variables|Electricity|SetisElectricityOn true)
  (Variables|Default|SetisGameOver false)
  (Variables|Default|SetisLookingAtPC false)
  (Variables|/Game/Blueprints/Main_Widget.Main_Widget_C|SetisGameOver _mainwidget false)
  (Variables|/Game/Blueprints/Main_Widget.Main_Widget_C|SetisPowerOff _mainwidget false)
  (Variables|/Game/Blueprints/Main_Widget.Main_Widget_C|SetUIVisible _mainwidget true)
  (Variables|Electricity|SetcurrElectricityTime (Math|Random|RandomFloatinRange (Variables|Electricity|GetminTimeBeforeElectricityOff) (Variables|Electricity|GetmaxTimeBeforeElectricityOff)))
  (bind _returnvalue (Actor|GetActorOfClass "/Game/Blueprints/BP_ComputerManager.BP_ComputerManager_C"))
  (Default|ResetGame _returnvalue)
  (Variables|/Script/Engine.PlayerController|SetbShowMouseCursor (Game|GetPlayerController 0) false))

(fn SetLightSourcesActive
  (params (value :type Boolean))
  (if value
    (for _array_element (Variables|Electricity|GetLightsources)
      (bind _aspoint_light (Utilities|Casting|CastToPointLight _array_element))
      (Rendering|Components|Light|SetIntensity (Variables|/Script/Engine.PointLight|GetPointLightComponent _aspoint_light) 25.0))
    (else
      (for _array_element_2 (Variables|Electricity|GetLightsources)
        (bind _aspoint_light_2 (Utilities|Casting|CastToPointLight _array_element_2))
        (Rendering|Components|Light|SetIntensity (Variables|/Script/Engine.PointLight|GetPointLightComponent _aspoint_light_2) 0.0)))))

(fn DecreaseElectricityTime
  (Variables|Electricity|SetcurrElectricityTime (- (Variables|Electricity|GetcurrElectricityTime) 1.0))
  (Variables|/Game/Blueprints/Main_Widget.Main_Widget_C|SetisPowerTimeDecreasing (Variables|Default|GetMainWidget) true)
  (Variables|Electricity|SetaccPowerTimeDecreasing 0.0))