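; BP_ComputerManager is an actor that controls which BP_Computer actors are active and runs the rig shop for buying more.
; On play and on reset only computer ID 1 is active; reset also restores each computer and the shop's index and price.
; The ToggleRigShop input shows or hides Widget_BuyRigs, toggling mouse cursor and character movement.
; ActivateComputer enables the computer matching an ID and adjusts the BP_GameMode balance by the price.
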(event EventBeginPlay
  (Utilities|FlowControl|Sequence
    (:then_0
      ;[1 1 1] Set Computers Active
      (bind _outactors (Actor|GetAllActorsOfClass "/Game/Blueprints/BP_Computer.BP_Computer_C"))
      (for _array_element _outactors
        (if (== (Variables|/Game/Blueprints/BP_Computer.BP_Computer_C|GetComputerId _array_element) 1)
          (Default|SetActive _array_element true)
          (else
            (Default|SetActive _array_element false)))))
    (:then_1
      (bind _returnvalue (UserInterface|CreateWidget "/Game/Blueprints/Widget_BuyRigs.Widget_BuyRigs_C"))
      (bind _output_get (Variables|Default|SetWidget _returnvalue))
      (Variables|/Game/Blueprints/Widget_BuyRigs.Widget_BuyRigs_C|SetComputerManager _output_get self))
    (:then_2
      (Input|EnableInput (Game|GetPlayerController 0)))))

(event Collision|EventActorBeginOverlap
  (params (OtherActor :type Actor%20Object%20Reference)))

(event EventTick
  (params (DeltaSeconds :type Float%20%28single-precision%29)))

(event Input|ActionEvents|InputActionToggleRigShop
  (params (Key :type Key%20Structure :default "None"))
  (bind _returnvalue (Game|GetPlayerCharacter 0))
  (bind _returnvalue_2 (Game|GetPlayerController 0))
  (bind _widget (Variables|Default|GetWidget))
  (:Released
    (if (Variables|Default|GetisOpen)
      (Variables|Default|SetisOpen false)
      (Widget|RemovefromParent _widget)
      (Variables|/Script/Engine.PlayerController|SetbShowMouseCursor _returnvalue_2 false)
      (bind _asbp_character (Utilities|Casting|CastToBP_Character _returnvalue))
      (Default|SetMovement _asbp_character true)
      (else
        (Variables|Default|SetisOpen true)
        (UserInterface|Viewport|AddtoViewport _widget 0)
        (Variables|/Script/Engine.PlayerController|SetbShowMouseCursor _returnvalue_2 true)
        (bind _asbp_character_2 (Utilities|Casting|CastToBP_Character _returnvalue))
        (Default|SetMovement _asbp_character_2 false)))))

(fn ConstructionScript)

(fn ActivateComputer
  (params (Index :type Integer) (Price :type Float%20%28single-precision%29))
  (bind _outactors (Actor|GetAllActorsOfClass "/Game/Blueprints/BP_Computer.BP_Computer_C"))
  (bind _result (Math|Integer|DecrementInt Index)
    (:%20%20
      (if (< (Utilities|Array|Length _outactors) _result)
        (return false)
        (else
          (bind _array_element (Utilities|Array|ForEachLoopwithBreak _outactors)
            (:LoopBody
              (if (== (Variables|/Game/Blueprints/BP_Computer.BP_Computer_C|GetComputerId _array_element) Index)
                (Default|SetActive _array_element true)
                (bind _asbp_game_mode (Utilities|Casting|CastToBP_GameMode (Game|GetGameMode)))
                (bind _result_2 (Math|Float|NegateFloat Price)
                  (:%20%20
                    (Default|AddBalance _asbp_game_mode _result_2)
                    (return true)))))))))))

(fn ResetGame
  (bind _widget (Variables|Default|GetWidget))
  (Utilities|FlowControl|Sequence
    (:then_0
      ;[1 1 1] Set Computers Active
      (bind _outactors (Actor|GetAllActorsOfClass "/Game/Blueprints/BP_Computer.BP_Computer_C"))
      (for _array_element _outactors
        (Default|ResetGame _array_element)
        (if (== (Variables|/Game/Blueprints/BP_Computer.BP_Computer_C|GetComputerId _array_element) 1)
          (Default|SetActive _array_element true)
          (else
            (Default|SetActive _array_element false)))))
    (:then_1
      ;[1 1 1] Restart UI
      (Variables|Default|SetisOpen false)
      (Variables|/Game/Blueprints/Widget_BuyRigs.Widget_BuyRigs_C|SetcurrIndex _widget 3)
      (Variables|/Game/Blueprints/Widget_BuyRigs.Widget_BuyRigs_C|SetcurrPrice _widget 1e+04))))