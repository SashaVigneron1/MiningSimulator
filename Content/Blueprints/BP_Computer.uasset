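; BP_Computer is an interactable PC actor that earns money for the GameManager from its installed CPU and GPU.
; All part variants spawn hidden at BeginPlay; buy functions charge once per part, then toggle visibility to swap it in.
; Tick pays income scaled by overclocking and doubled for matching brands; overclocking drives temperature, and overheating halts income with smoke until cooled.
; Interacting nearby moves the player camera to the screen and opens Widget_Computer.
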(event EventTick
  (params (DeltaSeconds :type Float%20%28single-precision%29))
  (bind _cpu (Variables|CurrEquipment|GetCPU))
  (bind _overclockingpercentage (Variables|Overclocking|GetOverclockingPercentage))
  (bind _gamemanager (Variables|Managers|GetGameManager))
  (bind _gpu (Variables|CurrEquipment|GetGPU))
  (bind _returnvalue (/ _overclockingpercentage 1e+02))
  (bind _cashpersecond (Variables|/Game/Blueprints/ComputerComponents/CPU/Base/BP_CPU.BP_CPU_C|GetCashPerSecond _cpu))
  (bind _cashpersecond_2 (Variables|/Game/Blueprints/ComputerComponents/GPU/Base/BP_GPU.BP_GPU_C|GetCashPerSecond _gpu))
  (bind _returnvalue_2 (+ _cashpersecond_2 _cashpersecond))
  (bind _returnvalue_3 (* _returnvalue_2 DeltaSeconds))
  (bind _returnvalue_4 (* _returnvalue_3 _returnvalue))
  (Utilities|FlowControl|Sequence
    (:then_0
      ;[1 1 1] Event Tick
      (if (Variables|Default|GetisActive)
        (if (not (Variables|/Game/Blueprints/Core/BP_GameMode.BP_GameMode_C|GetisGameOver _gamemanager))
          (if (Variables|/Game/Blueprints/Core/BP_GameMode.BP_GameMode_C|GetisElectricityOn _gamemanager)
            (if (not (Variables|Overclocking|GethasCrashed))
              (if (< (Variables|Overclocking|GetTemperature) 99.0)
                ;;[1 1 1] Get Profit
                (if (!= _cpu 0)
                  (if (!= _gpu 0)
                    ;;[1 1 1] Add Multiplier
                    (if (Utilities|Enum|Equal(Enum) (Variables|/Game/Blueprints/ComputerComponents/GPU/Base/BP_GPU.BP_GPU_C|GetBrand _gpu) (Variables|/Game/Blueprints/ComputerComponents/CPU/Base/BP_CPU.BP_CPU_C|GetBrand _cpu))
                      (Default|AddBalance (Variables|Managers|GetGameManager) (* _returnvalue_4 2.0))
                      (else
                        (Default|AddBalance (Variables|Managers|GetGameManager) _returnvalue_4)))
                    ;;[1 1 1] Overclocking Increase Temperature
                    (if (> (Variables|Overclocking|GetOverclockingPercentage) 8e+01)
                      (Variables|Overclocking|SetTemperature (+ (Variables|Overclocking|GetTemperature) (* DeltaSeconds (* (Math|Float|MakeLiteralFloat 1.0) (/ (Variables|Overclocking|GetOverclockingPercentage) 1e+02)))))
                      (else
                        ;;[1 1 1] Overclocking Decrease Temperature
                        (if (and (< (Variables|Overclocking|GetOverclockingPercentage) 8e+01) (> (Variables|Overclocking|GetTemperature) 6e+01))
                          (Variables|Overclocking|SetTemperature (+ (Variables|Overclocking|GetTemperature) (* DeltaSeconds (* (Math|Float|MakeLiteralFloat -1.0) (/ (- (Math|Float|MakeLiteralFloat 1e+02) (Variables|Overclocking|GetOverclockingPercentage)) 1e+02))))))))))
                (else
                  (Variables|Overclocking|SetTemperature (- (Variables|Overclocking|GetTemperature) DeltaSeconds))
                  (Variables|Overclocking|SethasCrashed true)
                  (bind _returnvalue_5 (Effects|SpawnEmitteratLocation "/Game/StarterContent/Particles/P_Smoke.P_Smoke" (Transformation|GetWorldLocation (Variables|Default|GetDefaultSceneRoot))))
                  (Variables|Default|SetParticles _returnvalue_5)))
              (else
                (Variables|Overclocking|SetTemperature (- (Variables|Overclocking|GetTemperature) DeltaSeconds) :!label _label)
                (if (< (Variables|Overclocking|GetTemperature) 8e+01)
                  (Variables|Overclocking|SethasCrashed false)
                  (Components|DestroyComponent (Variables|Default|GetParticles)))))
            (elif (Variables|Overclocking|GethasCrashed)
              (goto _label))))))
    (:then_1
      ;[1 1 1] Set Interactable
      (bind _output_get (Variables|Default|Setinteractable (and (Variables|Default|GetisActive) (and (not (Variables|/Game/Blueprints/Core/BP_GameMode.BP_GameMode_C|GetisLookingAtPC (Variables|Managers|GetGameManager))) (< (Math|Vector|Distance2D(Vector) (Transformation|GetWorldLocation (Variables|Default|GetDefaultSceneRoot)) (Transformation|GetWorldLocation (Variables|/Script/Engine.Character|GetCapsuleComponent (Game|GetPlayerCharacter 0)))) 2e+02)))))
      (Default|SetInteractable (Variables|Default|GetInteractWidget) _output_get))))

(event EventBeginPlay
  (bind _gputransform (Variables|Default|GetGPUTransform))
  (bind _cputransform (Variables|Default|GetCPUTransform))
  (bind _returnvalue (Transformation|GetWorldTransform _cputransform))
  (bind _returnvalue_2 (Transformation|GetWorldTransform _gputransform))
  ;[1 1 1] Iniitalize
  (Utilities|FlowControl|Sequence
    (:then_0
      (Input|EnableInput (Game|GetPlayerController 0)))
    (:then_1
      ;;[1 1 1] Create Widget
      (bind _returnvalue_3 (UserInterface|CreateWidget "/Game/Blueprints/Widget_Computer.Widget_Computer_C"))
      (bind _output_get (Variables|Managers|SetWidget _returnvalue_3))
      (Default|SetPC _output_get self))
    (:then_2
      (bind _asbp_game_mode (Utilities|Casting|CastToBP_GameMode (Game|GetGameMode)))
      (Variables|Managers|SetGameManager _asbp_game_mode))
    (:then_3
      ;;[1 1 1] Create Objects
      ;;;[1 1 1] Create GPUs
      (bind _returnvalue_4 (Game|SpawnActorfromClass "/Game/Blueprints/ComputerComponents/GPU/BP_GPU_Azur.BP_GPU_Azur_C" _returnvalue_2 "Undefined" 0 0))
      (bind _output_get_2 (Variables|GPUs|SetAzurGPU _returnvalue_4))
      (Rendering|SetVisibility (Variables|/Game/Blueprints/ComputerComponents/GPU/Base/BP_GPU.BP_GPU_C|GetCube _output_get_2) false false))
    (:then_4
      (bind _returnvalue_5 (Game|SpawnActorfromClass "/Game/Blueprints/ComputerComponents/GPU/BP_GPU_NSI.BP_GPU_NSI_C" _returnvalue_2 "Undefined" 0 0))
      (bind _output_get_3 (Variables|GPUs|SetNSIGPU _returnvalue_5))
      (Rendering|SetVisibility (Variables|/Game/Blueprints/ComputerComponents/GPU/Base/BP_GPU.BP_GPU_C|GetCube _output_get_3) false false))
    (:then_5
      (bind _returnvalue_6 (Game|SpawnActorfromClass "/Game/Blueprints/ComputerComponents/GPU/BP_GPU_ROG.BP_GPU_ROG_C" _returnvalue_2 "Undefined" 0 0))
      (bind _output_get_4 (Variables|GPUs|SetROGGPU _returnvalue_6))
      (Rendering|SetVisibility (Variables|/Game/Blueprints/ComputerComponents/GPU/Base/BP_GPU.BP_GPU_C|GetCube _output_get_4) false false))
    (:then_6
      ;;;[1 1 1] Create CPUs
      (bind _returnvalue_7 (Game|SpawnActorfromClass "/Game/Blueprints/ComputerComponents/CPU/BP_Azur_Zen3.BP_Azur_Zen3_C" _returnvalue "Undefined" 0 0))
      (bind _output_get_5 (Variables|CPUs|SetAzurCPU _returnvalue_7))
      (Rendering|SetVisibility (Variables|/Game/Blueprints/ComputerComponents/CPU/Base/BP_CPU.BP_CPU_C|GetCube _output_get_5) false false))
    (:then_7
      (bind _returnvalue_8 (Game|SpawnActorfromClass "/Game/Blueprints/ComputerComponents/CPU/BP_NSI_I9.BP_NSI_I9_C" _returnvalue "Undefined" 0 0))
      (bind _output_get_6 (Variables|CPUs|SetNSICPU _returnvalue_8))
      (Rendering|SetVisibility (Variables|/Game/Blueprints/ComputerComponents/CPU/Base/BP_CPU.BP_CPU_C|GetCube _output_get_6) false false))
    (:then_8
      (bind _returnvalue_9 (Game|SpawnActorfromClass "/Game/Blueprints/ComputerComponents/CPU/BP_ROG_ThreadRipper.BP_ROG_ThreadRipper_C" _returnvalue "Undefined" 0 0))
      (bind _output_get_7 (Variables|CPUs|SetROGCPU _returnvalue_9))
      (Rendering|SetVisibility (Variables|/Game/Blueprints/ComputerComponents/CPU/Base/BP_CPU.BP_CPU_C|GetCube _output_get_7) false false))
    (:then_9
      (bind _returnvalue_10 (UserInterface|CreateWidget "/Game/Blueprints/InteractWidget.InteractWidget_C"))
      (bind _output_get_8 (Variables|Default|SetInteractWidget _returnvalue_10))
      (UserInterface|Viewport|AddtoViewport _output_get_8 0))))

(event Input|ActionEvents|InputActionResetCamera
  (params (Key :type Key%20Structure :default "None"))
  (bind _gamemanager (Variables|Managers|GetGameManager))
  ;[1 1 1] Reset Camera
  (:Released
    (if (Variables|Default|GetisActive)
      (if (Variables|CameraTransition|GetisLookingAtPC)
        (Utilities|FlowControl|Sequence
          (:then_0
            ;;[1 1 1] Zoom back out
            (if (Variables|CameraTransition|GetisCameraSet)
              (bind _asbp_character (Utilities|Casting|CastToBP_Character (Game|GetPlayerCharacter 0)))
              (bind _camera (Default|GetCamera _asbp_character))
              (Default|SetMovement _asbp_character true)
              (Transformation|SetWorldLocation _camera (Variables|CameraTransition|GetCameraOldPos) false false)
              (Transformation|SetWorldRotation _camera (Variables|CameraTransition|GetCameraOldRot) false false)
              (Variables|CameraTransition|SetisCameraSet false)))
          (:then_1
            (Widget|RemovefromParent (Variables|Managers|GetWidget)))
          (:then_2
            (bind _output_get (Variables|CameraTransition|SetisLookingAtPC false))
            (Variables|/Game/Blueprints/Core/BP_GameMode.BP_GameMode_C|SetisLookingAtPC _gamemanager _output_get)
            (Default|SetUIVisibility _gamemanager true)
            (Variables|/Script/Engine.PlayerController|SetbShowMouseCursor (Game|GetPlayerController 0) false)))))))

(event Input|ActionEvents|InputActionInteract
  (params (Key :type Key%20Structure :default "None"))
  (bind _cameratransform (Variables|Default|GetCameraTransform))
  (bind _gamemanager (Variables|Managers|GetGameManager))
  ;[1 1 1] Set Camera
  (:Pressed
    (if (not (Variables|/Game/Blueprints/Core/BP_GameMode.BP_GameMode_C|GetisLookingAtPC (Variables|Managers|GetGameManager)))
      (if (and (Variables|Default|GetisActive) (Variables|Default|Getinteractable))
        (if (not (Variables|CameraTransition|GetisLookingAtPC))
          (Utilities|FlowControl|Sequence
            (:then_0
              ;;[1 1 1] Zoom in to PC
              (if (not (Variables|CameraTransition|GetisCameraSet))
                ;;;[1 1 1] Get Camera
                (bind _asbp_character (Utilities|Casting|CastToBP_Character (Game|GetPlayerCharacter 0)))
                (bind _camera (Default|GetCamera _asbp_character))
                (Default|SetMovement _asbp_character false)
                ;;;[1 1 1] Set Old Position And Rotation
                (Variables|CameraTransition|SetCameraOldPos (Transformation|GetWorldLocation _camera))
                (Variables|CameraTransition|SetCameraOldRot (Transformation|GetWorldRotation _camera))
                (Transformation|SetWorldLocation _camera (Transformation|GetWorldLocation _cameratransform) false false)
                (Transformation|SetWorldRotation _camera (Transformation|GetWorldRotation _cameratransform) false false)
                (Variables|CameraTransition|SetisCameraSet true)))
            (:then_1
              (UserInterface|Viewport|AddtoViewport (Variables|Managers|GetWidget) 0))
            (:then_2
              (bind _output_get (Variables|CameraTransition|SetisLookingAtPC true))
              (Variables|/Game/Blueprints/Core/BP_GameMode.BP_GameMode_C|SetisLookingAtPC _gamemanager _output_get)
              (Default|SetUIVisibility _gamemanager false)
              (Variables|/Script/Engine.PlayerController|SetbShowMouseCursor (Game|GetPlayerController 0) true))))))))

(fn ConstructionScript)

(fn BuyAzurGPU
  (bind _azurgpu (Variables|GPUs|GetAzurGPU))
  (if (Variables|GPUs|GethasAzurGPU)
    _
    (else
      (Default|AddBalance (Variables|Managers|GetGameManager) -4e+03)
      (Variables|GPUs|SethasAzurGPU true)
      (Audio|PlaySound2D "/Game/Sounds/Purchase.Purchase" 1.0 1.0 0.0 0 0)))
  (if (!= (Variables|CurrEquipment|GetGPU) 0)
    (Rendering|SetVisibility (Variables|/Game/Blueprints/ComputerComponents/GPU/Base/BP_GPU.BP_GPU_C|GetCube (Variables|CurrEquipment|GetGPU)) false false))
  (Rendering|SetVisibility (Variables|/Game/Blueprints/ComputerComponents/GPU/Base/BP_GPU.BP_GPU_C|GetCube _azurgpu) true false)
  (bind _output_get (Variables|CurrEquipment|SetGPU _azurgpu))
  (Default|SetGPU (Variables|Managers|GetWidget) _output_get))

(fn BuyAzurCPU
  (if (Variables|CPUs|GethasAzurCPU)
    _
    (else
      (Default|AddBalance (Variables|Managers|GetGameManager) -4e+03)
      (Variables|CPUs|SethasAzurCPU true)
      (Audio|PlaySound2D "/Game/Sounds/Purchase.Purchase" 1.0 1.0 0.0 0 0)))
  (if (!= (Variables|CurrEquipment|GetCPU) 0)
    (Rendering|SetVisibility (Variables|/Game/Blueprints/ComputerComponents/CPU/Base/BP_CPU.BP_CPU_C|GetCube (Variables|CurrEquipment|GetCPU)) false false))
  (Rendering|SetVisibility (Variables|/Game/Blueprints/ComputerComponents/CPU/Base/BP_CPU.BP_CPU_C|GetCube (Variables|CPUs|GetAzurCPU)) true false)
  (bind _output_get (Variables|CurrEquipment|SetCPU (Variables|CPUs|GetAzurCPU)))
  (Default|SetCPU (Variables|Managers|GetWidget) _output_get))

(fn BuyNSIGPU
  (bind _nsigpu (Variables|GPUs|GetNSIGPU))
  (if (Variables|GPUs|GethasNSIGPU)
    _
    (else
      (Default|AddBalance (Variables|Managers|GetGameManager) -1e+04)
      (Variables|GPUs|SethasNSIGPU true)
      (Audio|PlaySound2D "/Game/Sounds/Purchase.Purchase" 1.0 1.0 0.0 0 0)))
  (Rendering|SetVisibility (Variables|/Game/Blueprints/ComputerComponents/GPU/Base/BP_GPU.BP_GPU_C|GetCube (Variables|CurrEquipment|GetGPU)) false false)
  (Rendering|SetVisibility (Variables|/Game/Blueprints/ComputerComponents/GPU/Base/BP_GPU.BP_GPU_C|GetCube _nsigpu) true false)
  (bind _output_get (Variables|CurrEquipment|SetGPU _nsigpu))
  (Default|SetGPU (Variables|Managers|GetWidget) _output_get))

(fn BuyNSICPU
  (bind _nsicpu (Variables|CPUs|GetNSICPU))
  (if (Variables|CPUs|GethasNSICPU)
    _
    (else
      (Default|AddBalance (Variables|Managers|GetGameManager) -1e+04)
      (Variables|CPUs|SethasNSICPU true)
      (Audio|PlaySound2D "/Game/Sounds/Purchase.Purchase" 1.0 1.0 0.0 0 0)))
  (Rendering|SetVisibility (Variables|/Game/Blueprints/ComputerComponents/CPU/Base/BP_CPU.BP_CPU_C|GetCube (Variables|CurrEquipment|GetCPU)) false false)
  (Rendering|SetVisibility (Variables|/Game/Blueprints/ComputerComponents/CPU/Base/BP_CPU.BP_CPU_C|GetCube _nsicpu) true false)
  (bind _output_get (Variables|CurrEquipment|SetCPU _nsicpu))
  (Default|SetCPU (Variables|Managers|GetWidget) _output_get))

(fn BuyROGGPU
  (bind _roggpu (Variables|GPUs|GetROGGPU))
  (if (Variables|GPUs|GethasROGGPU)
    _
    (else
      (Default|AddBalance (Variables|Managers|GetGameManager) -2.5e+04)
      (Variables|GPUs|SethasROGGPU true)
      (Audio|PlaySound2D "/Game/Sounds/Purchase.Purchase" 1.0 1.0 0.0 0 0)))
  (if (!= (Variables|CurrEquipment|GetGPU) 0)
    (Rendering|SetVisibility (Variables|/Game/Blueprints/ComputerComponents/GPU/Base/BP_GPU.BP_GPU_C|GetCube (Variables|CurrEquipment|GetGPU)) false false))
  (Rendering|SetVisibility (Variables|/Game/Blueprints/ComputerComponents/GPU/Base/BP_GPU.BP_GPU_C|GetCube _roggpu) true false)
  (bind _output_get (Variables|CurrEquipment|SetGPU _roggpu))
  (Default|SetGPU (Variables|Managers|GetWidget) _output_get))

(fn BuyROGCPU
  (bind _rogcpu (Variables|CPUs|GetROGCPU))
  (if (Variables|CPUs|GethasROGCPU)
    _
    (else
      (Default|AddBalance (Variables|Managers|GetGameManager) -2.5e+04)
      (Variables|CPUs|SethasROGCPU true)
      (Audio|PlaySound2D "/Game/Sounds/Purchase.Purchase" 1.0 1.0 0.0 0 0)))
  (if (!= (Variables|CurrEquipment|GetCPU) 0)
    (Rendering|SetVisibility (Variables|/Game/Blueprints/ComputerComponents/CPU/Base/BP_CPU.BP_CPU_C|GetCube (Variables|CurrEquipment|GetCPU)) false false))
  (Rendering|SetVisibility (Variables|/Game/Blueprints/ComputerComponents/CPU/Base/BP_CPU.BP_CPU_C|GetCube _rogcpu) true false)
  (bind _output_get (Variables|CurrEquipment|SetCPU _rogcpu))
  (Default|SetCPU (Variables|Managers|GetWidget) _output_get))

(fn SetActive
  (params (value :type Boolean))
  (bind _gpu (Variables|CurrEquipment|GetGPU))
  (bind _cpu (Variables|CurrEquipment|GetCPU))
  (bind _cpu_2 (Variables|CurrEquipment|GetCPU))
  (bind _gpu_2 (Variables|CurrEquipment|GetGPU))
  (if value
    (Variables|Default|SetisActive true)
    (if (!= _gpu 0)
      (Rendering|SetVisibility (Variables|/Game/Blueprints/ComputerComponents/GPU/Base/BP_GPU.BP_GPU_C|GetCube _gpu) true false))
    (if (!= _cpu_2 0)
      (Rendering|SetVisibility (Variables|/Game/Blueprints/ComputerComponents/CPU/Base/BP_CPU.BP_CPU_C|GetCube _cpu_2) true false))
    (Rendering|SetVisibility (Variables|Default|GetPC) true false)
    (else
      (Variables|Default|SetisActive false)
      (if (!= _gpu_2 0)
        (Rendering|SetVisibility (Variables|/Game/Blueprints/ComputerComponents/GPU/Base/BP_GPU.BP_GPU_C|GetCube _gpu_2) false false))
      (if (!= _cpu 0)
        (Rendering|SetVisibility (Variables|/Game/Blueprints/ComputerComponents/CPU/Base/BP_CPU.BP_CPU_C|GetCube _cpu) false false))
      (Rendering|SetVisibility (Variables|Default|GetPC) false false))))

(fn GetRevenue
  (bind _cpu (Variables|CurrEquipment|GetCPU))
  (bind _overclockingpercentage (Variables|Overclocking|GetOverclockingPercentage))
  (bind _gpu (Variables|CurrEquipment|GetGPU))
  (bind _returnvalue (/ _overclockingpercentage 1e+02))
  (bind _cashpersecond (Variables|/Game/Blueprints/ComputerComponents/GPU/Base/BP_GPU.BP_GPU_C|GetCashPerSecond _gpu))
  (bind _cashpersecond_2 (Variables|/Game/Blueprints/ComputerComponents/CPU/Base/BP_CPU.BP_CPU_C|GetCashPerSecond _cpu))
  (bind _returnvalue_2 (+ _cashpersecond _cashpersecond_2))
  (bind _returnvalue_3 (* _returnvalue_2 1.0))
  (bind _returnvalue_4 (* _returnvalue_3 _returnvalue))
  ;[1 1 1] Event Tick
  (if (Variables|Default|GetisActive)
    (Utilities|FlowControl|Sequence
      (:then_0
        (if (not (Variables|Overclocking|GethasCrashed))
          ;;[1 1 1] Get Profit
          (if (!= _cpu 0)
            (if (!= _gpu 0)
              ;;[1 1 1] Add Multiplier
              (if (Utilities|Enum|Equal(Enum) (Variables|/Game/Blueprints/ComputerComponents/GPU/Base/BP_GPU.BP_GPU_C|GetBrand _gpu) (Variables|/Game/Blueprints/ComputerComponents/CPU/Base/BP_CPU.BP_CPU_C|GetBrand _cpu))
                (return (* _returnvalue_4 2.0))
                (else
                  (return _returnvalue_4)))
              (else
                _)))))))
  (return 0.0))

(fn ResetGame
  (bind _gamemanager (Variables|Managers|GetGameManager))
  (Utilities|FlowControl|Sequence
    (:then_0
      (Variables|Overclocking|SetTemperature 6e+01)
      (Variables|Overclocking|SetOverclockingPercentage 8e+01))
    (:then_1
      (Variables|CPUs|SethasAzurCPU false)
      (Variables|GPUs|SethasAzurGPU false))
    (:then_2
      (Variables|CPUs|SethasNSICPU false)
      (Variables|GPUs|SethasNSIGPU false))
    (:then_3
      (Variables|CPUs|SethasROGCPU false)
      (Variables|GPUs|SethasROGGPU false))
    (:then_4
      ;[1 1 1] ResetCamera
      (if (Variables|Default|GetisActive)
        (if (Variables|CameraTransition|GetisLookingAtPC)
          (Utilities|FlowControl|Sequence
            (:then_0
              ;;[1 1 1] Zoom back out
              (if (Variables|CameraTransition|GetisCameraSet)
                (bind _asbp_character (Utilities|Casting|CastToBP_Character (Game|GetPlayerCharacter 0)))
                (bind _camera (Default|GetCamera _asbp_character))
                (Default|SetMovement _asbp_character true)
                (Transformation|SetWorldLocation _camera (Variables|CameraTransition|GetCameraOldPos) false false)
                (Transformation|SetWorldRotation _camera (Variables|CameraTransition|GetCameraOldRot) false false)
                (Variables|CameraTransition|SetisCameraSet false)))
            (:then_1
              (Widget|RemovefromParent (Variables|Managers|GetWidget)))
            (:then_2
              (bind _output_get (Variables|CameraTransition|SetisLookingAtPC false))
              (Variables|/Game/Blueprints/Core/BP_GameMode.BP_GameMode_C|SetisLookingAtPC _gamemanager _output_get)
              (Default|SetUIVisibility _gamemanager true)
              (Variables|/Script/Engine.PlayerController|SetbShowMouseCursor (Game|GetPlayerController 0) false))))))
    (:then_5
      (Variables|CameraTransition|SetisLookingAtPC false))
    (:then_6
      (if (!= (Variables|CurrEquipment|GetCPU) 0)
        (Rendering|SetVisibility (Variables|/Game/Blueprints/ComputerComponents/CPU/Base/BP_CPU.BP_CPU_C|GetCube (Variables|CurrEquipment|GetCPU)) false false)))
    (:then_7
      (if (!= (Variables|CurrEquipment|GetGPU) 0)
        (Rendering|SetVisibility (Variables|/Game/Blueprints/ComputerComponents/GPU/Base/BP_GPU.BP_GPU_C|GetCube (Variables|CurrEquipment|GetGPU)) false false)))
    (:then_8
      (Variables|CurrEquipment|SetCPU 0)
      (Variables|CurrEquipment|SetGPU 0))))