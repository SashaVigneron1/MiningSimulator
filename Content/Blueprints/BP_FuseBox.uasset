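; BP_FuseBox is an interactable fuse box that the player can use while the game mode's electricity is off.
; Tick lights its point light during an outage and enables its own interact widget when the player is within horizontal range.
; Pressing Interact then calls DecreaseElectricityTime on BP_GameMode, plays a fuse-fix sound and spawns a small explosion effect.
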(event EventBeginPlay
  (Utilities|FlowControl|Sequence
    (:then_0
      (Input|EnableInput (Game|GetPlayerController 0)))
    (:then_1
      (bind _returnvalue (UserInterface|CreateWidget "/Game/Blueprints/InteractWidget.InteractWidget_C"))
      (bind _output_get (Variables|Default|SetInteractWidget _returnvalue))
      (UserInterface|Viewport|AddtoViewport _output_get 0))
    (:then_2
      (bind _asbp_game_mode (Utilities|Casting|CastToBP_GameMode (Game|GetGameMode)))
      (Variables|Default|SetGameMode _asbp_game_mode))
    (:then_3
      (Rendering|Components|Light|SetIntensity (Variables|Default|GetPointLight) 0.0))))

(event EventTick
  (params (DeltaSeconds :type Float%20%28single-precision%29))
  (bind _gamemode (Variables|Default|GetGameMode))
  (bind _iselectricityon (Variables|/Game/Blueprints/Core/BP_GameMode.BP_GameMode_C|GetisElectricityOn _gamemode))
  (bind _returnvalue (not _iselectricityon))
  ;[1 1 1] Set Interactability
  (if _returnvalue
    (Rendering|Components|Light|SetIntensity (Variables|Default|GetPointLight) 5e+03)
    (bind _output_get (Variables|Default|SetcanInteract (and _returnvalue (< (Math|Vector|Distance2D(Vector) (Transformation|GetWorldLocation (Variables|Default|GetDefaultSceneRoot)) (Transformation|GetWorldLocation (Variables|/Script/Engine.Character|GetCapsuleComponent (Game|GetPlayerCharacter 0)))) 5e+02))))
    (Variables|/Game/Blueprints/InteractWidget.InteractWidget_C|Setinteractable (Variables|Default|GetInteractWidget) _output_get)
    (else
      (Rendering|Components|Light|SetIntensity (Variables|Default|GetPointLight) 0.0)
      (bind _output_get_2 (Variables|Default|SetcanInteract false))
      (Variables|/Game/Blueprints/InteractWidget.InteractWidget_C|Setinteractable (Variables|Default|GetInteractWidget) _output_get_2))))

(event Input|ActionEvents|InputActionInteract
  (params (Key :type Key%20Structure :default "None"))
  ;[1 1 1] Interact
  (:Pressed
    (if (Variables|Default|GetcanInteract)
      (Default|DecreaseElectricityTime (Variables|Default|GetGameMode))
      (Audio|PlaySound2D "/Game/Sounds/FuseFix.FuseFix" 1.0 1.0 1.5 0 0)
      (Effects|SpawnEmitteratLocation "/Game/StarterContent/Particles/P_Explosion.P_Explosion" (+ (Transformation|GetWorldLocation (Variables|Default|GetDefaultSceneRoot)) "0.000000,50.000000,100.000000") "0, 0, 0" "0.100000,0.100000,0.100000"))))

(fn ConstructionScript)